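; BP_EnemyBasic is a creep that moves along the first BP_Spline each tick, damaging BPI_HittedPlayer actors on overlap, then destroying itself.
; Damage events reduce life; DamageOverTime also starts slow/freeze and a recursive DoT loop, which decrements but never checks its tick count.
; Freeze without slow never restores speed.
; Death spawns particles, hides the enemy, notifies BP_EnemySpawner, then destroys it after a delay.
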(event OnComponentBeginOverlap(EnemyBase)
  (params (OverlappedComponent :type Primitive%20Component%20Object%20Reference) (OtherActor :type Actor%20Object%20Reference) (OtherComp :type Primitive%20Component%20Object%20Reference) (OtherBodyIndex :type Integer) (bFromSweep :type Boolean) (SweepResult :type Hit%20Result%20Structure%20%28by%20ref%29))
  ;[1 1 1] Hit Player
  (if (Utilities|DoesObjectImplementInterface OtherActor "/Game/BluePrints/BPI_HittedPlayer.BPI_HittedPlayer_C")
    (Class|BPIHittedPlayer|HitPlayer(Message) OtherActor (Variables|Default|GetE_Damage))
    (Utilities|FlowControl|Delay 0.2)
    (Actor|DestroyActor)))

(event Custom|DotLoop
  (Variables|Default|SetE_Life (- (Variables|Default|GetE_Life) (Variables|Default|GetTickDamage)))
  (Utilities|FlowControl|Delay (Variables|Default|GetIntervall))
  (Variables|Default|SetCountDot (- (Variables|Default|GetCountDot) 1))
  (if (<= (Variables|Default|GetE_Life) 0.0)
    (CallFunction|EnemyDeath)
    (else
      (CallFunction|DotLoop))))

(event Custom|Dot
  (params (DotDuration :type Float%20%28single-precision%29) (DotDamage :type Float%20%28single-precision%29) (DotTicks :type Integer))
  (bind _returnvalue (Math|Conversions|ToFloat(Integer) DotTicks))
  (Variables|Default|SetCountDot DotTicks)
  (Variables|Default|SetIntervall (/ DotDuration _returnvalue))
  (Variables|Default|SetTickDamage (/ DotDamage _returnvalue))
  (Variables|Default|SetE_Life (- (Variables|Default|GetE_Life) (Variables|Default|GetTickDamage)))
  (Utilities|FlowControl|Delay (Variables|Default|GetIntervall))
  (Variables|Default|SetCountDot (- (Variables|Default|GetCountDot) 1))
  (if (<= (Variables|Default|GetE_Life) 0.0)
    (CallFunction|EnemyDeath)
    (else
      (CallFunction|DotLoop))))

(event Custom|EnemyDeath
  ;[1 1 1] CreateCustomEvent::Destroy Actor and Play Death Particle System
  (Effects|SpawnEmitteratLocation "/Game/Particles/Creeps/PS_CreepDeath.PS_CreepDeath" (Transformation|GetWorldLocation (Variables|Default|GetParticleSpawnLocation)))
  (Variables|Default|SetE_Speed 0.005)
  (Rendering|SetVisibility (Variables|Default|GetEnemyBase) false false)
  (Collision|SetCollisionEnabled (Variables|Default|GetEnemyBase) "NoCollision")
  (Rendering|SetVisibility (Variables|Default|Get3d_fast_worm_low_complete) false false)
  (Collision|SetCollisionEnabled (Variables|Default|Get3d_fast_worm_low_complete) "NoCollision")
  (bind _outactors (Actor|GetAllActorsOfClass "/Game/BluePrints/BP_EnemySpawner.BP_EnemySpawner_C"))
  (Utilities|FlowControl|Sequence
    (:then_0
      (Utilities|FlowControl|Delay 4.05)
      (Actor|DestroyActor))
    (:then_1
      (Utilities|FlowControl|DoOnce false
        (:Completed
          (Default|CountEnemysLeft (Utilities|Array|Get(acopy) _outactors)))))))

(event Custom|Slow
  (params (SlowDuration :type Float%20%28single-precision%29) (SpeedMultiplier :type Float%20%28single-precision%29) (FreezDuration :type Float%20%28single-precision%29))
  (if (> FreezDuration 0.0)
    (Variables|Default|SetE_Speed 0.0)
    (Utilities|FlowControl|Delay FreezDuration))
  (if (> SlowDuration 0.0)
    (Variables|Default|SetE_Speed (* (Variables|Default|GetDefaultSpeed) SpeedMultiplier))
    (Utilities|FlowControl|Delay SlowDuration)
    (Variables|Default|SetE_Speed (Variables|Default|GetDefaultSpeed))))

(event EventDamageValue
  (params (Damage :type Float%20%28single-precision%29))
  (bind _output_get (Variables|Default|SetE_Life (- (Variables|Default|GetE_Life) Damage)))
  (if (<= _output_get 0.0)
    (CallFunction|EnemyDeath)))

(event EventTick
  (params (DeltaSeconds :type Float%20%28single-precision%29))
  (bind _storedspline (Variables|Default|GetStoredSpline))
  (Variables|Default|SetStoredDistance (+ (Variables|Default|GetE_Speed) (Variables|Default|GetStoredDistance)))
  (Transformation|SetWorldLocationAndRotation (Variables|Default|GetDefaultSceneRoot) (Spline|GetLocationatDistanceAlongSpline _storedspline (Variables|Default|GetStoredDistance) "World") (Spline|GetRotationatDistanceAlongSpline _storedspline (Variables|Default|GetStoredDistance) "World") false false))

(event EventAreaDamage
  (params (Damage :type Float%20%28single-precision%29))
  (bind _output_get (Variables|Default|SetE_Life (- (Variables|Default|GetE_Life) Damage)))
  (if (<= _output_get 0.0)
    (CallFunction|EnemyDeath)))

(event EventDamageOverTime
  (params (DotDuration :type Float%20%28single-precision%29) (DotDamage :type Float%20%28single-precision%29) (DOTTicks :type Integer) (SlowDuration :type Float%20%28single-precision%29) (SpeedMultiplier :type Float%20%28single-precision%29) (FreezDuration :type Float%20%28single-precision%29))
  (Utilities|FlowControl|Sequence
    (:then_0
      (if (> DotDuration 0.0)
        (CallFunction|Dot DotDuration DotDamage DOTTicks)))
    (:then_1
      (if (or (> SlowDuration 0.0) (> FreezDuration 0.0))
        (CallFunction|Slow SlowDuration SpeedMultiplier FreezDuration)))))

(event EventBeginPlay
  (bind _outactors (Actor|GetAllActorsOfClass "/Game/BluePrints/BP_Spline.BP_Spline_C"))
  (Variables|Default|SetStoredSpline (Variables|/Game/BluePrints/BP_Spline.BP_Spline_C|GetSpline (Utilities|Array|Get(acopy) _outactors))))

(fn ConstructionScript
  (Variables|Default|SetDefaultSpeed (Variables|Default|GetE_Speed)))