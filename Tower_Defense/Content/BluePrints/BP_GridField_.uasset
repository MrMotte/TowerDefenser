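; Tappable tower-defense grid cell that opens a radial menu for placing or replacing a tower, or plays a sprite fade if marked as an obstacle.
; A tap first dismisses any open radial menu and suppresses tower colliders; otherwise it highlights the cell and passes the tower's class name or "Default" to a new menu.
; The menu calls back to swap the tower or restore the cell's look, and Level 1 taps notify the tutorial.
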(event OnInputTouchBegin(Cell)
  (params (FingerIndex :type ETouchIndex%20Enum :default "Touch1") (TouchedComponent :type Primitive%20Component%20Object%20Reference))
  ;[0.3185 0 1 1 30] Clean Widgets, Create Obstacle OR Radial Menu
  (bind _foundwidgets (Widget|GetAllWidgetsOfClass "/Game/BluePrints/UI/BP_Radial.BP_Radial_C" true))
  (Utilities|IsValid (Utilities|Array|Get(acopy) _foundwidgets)
    (:Is%20Valid
      (for _array_element _foundwidgets
        (Widget|RemovefromParent _array_element)
        (CallFunction|GetAllTowersandSuspressCollider)))
    (:Is%20Not%20Valid
      (if (Variables|Default|GetIsObstacle)
        (bind _alpha (Timeline|FadeOut PlayFromStart)
          (:Update
            (CallFunction|SetColorOfObstacle _alpha)))
        (else
          (Utilities|FlowControl|Sequence
            (:then_0
              (CallFunction|CreateRadialMenuWidget)
              (Utilities|IsValid (Variables|Default|GetPlacedTower)
                (:Is%20Valid
                  (CallFunction|GetPlacedTowerClassNameandSendtoRadialMenu)
                  (Class|BPIShoot|ShowCollider(Message) (Variables|Default|GetPlacedTower)))
                (:Is%20Not%20Valid
                  (CallFunction|Send"Default"toRadialMenu))))
            (:then_1
              (CallFunction|TutorialTriggerLevel1))))))))

(event Custom|TutorialTriggerLevel1
  (bind _asbp_character (Utilities|Casting|CastToBP_Character (Game|Player|GetPlayerPawn 0)))
  (if (Utilities|Enum|Equal(Enum) (Variables|/Game/BluePrints/BP_Character.BP_Character_C|GetLevelNameGameplay _asbp_character) "Level1_Gameplay")
    (Utilities|FlowControl|DoOnce false
      (:Completed
        (bind _foundwidgets (Widget|GetAllWidgetsOfClass "/Game/BluePrints/UI/BP_Tutorial.BP_Tutorial_C" true))
        (Utilities|IsValid (Utilities|Array|Get(acopy) _foundwidgets)
          (:Is%20Valid
            (Default|TappedGrid (Utilities|Array|Get(acopy) _foundwidgets))))))))

(event EventRadialMenuClosed
  (bind _output_get (Variables|Default|SetCell (Variables|Default|GetCell)))
  (Sprite|SetSpriteColor _output_get (Math|Conversions|ToLinearColor(Color) (Variables|Default|GetAvailableCellColor))) ; Auswählbare Grid-Felder in der Farbe Available Cell Color einfärben
  (Rendering|Components|Sprite|SetSprite (Variables|Default|GetCell) (Variables|Default|GetAvailableCellSprite)))

(event EventBeginPlay
  (bind _foundwidgets (Widget|GetAllWidgetsOfClass "/Game/BluePrints/UI/BP_Radial.BP_Radial_C" true))
  (Utilities|IsValid (Utilities|Array|Get(acopy) _foundwidgets)
    (:Is%20Not%20Valid
      (if (Variables|Default|GetIsObstacle)
        (bind _output_get (Variables|Default|SetCell (Variables|Default|GetCell)))
        (Sprite|SetSpriteColor _output_get "(R=0.000000,G=0.000000,B=0.000000,A=0.000000)") ; Nicht auswählbare Grid-Felder unsichtbar schalten
        (else
          (bind _output_get_2 (Variables|Default|SetCell (Variables|Default|GetCell)))
          (Sprite|SetSpriteColor _output_get_2 (Math|Conversions|ToLinearColor(Color) (Variables|Default|GetAvailableCellColor))) ; Auswählbare Grid-Felder in der Farbe Available Cell Color einfärben
          (Rendering|Components|Sprite|SetSprite (Variables|Default|GetCell) (Variables|Default|GetAvailableCellSprite)))))))

(event EventButtonClicked
  (params (New%20Tower%20Class :type Actor%20Class%20Reference))
  ;[1 0 1 1 30] Get Interface Event (Button click on selected Tower) from Radial Menu, delete old Tower and spawn new
  (Variables|Default|SetChoosenClass New%20Tower%20Class)
  (Actor|DestroyActor (Variables|Default|GetPlacedTower))
  (bind _returnvalue (Game|SpawnActorfromClass (Variables|Default|GetChoosenClass) (Math|Transform|MakeTransform (.Location (Math|Transform|BreakTransform (Transformation|GetWorldTransform (Variables|Default|GetDefaultSceneRoot))))) "AlwaysSpawn" 0 0))
  (Variables|Default|SetPlacedTower _returnvalue))

(fn ConstructionScript)

(fn GetPlacedTowerClassNameandSendtoRadialMenu
  (bind _output_get (Variables|Default|SetClass (Utilities|GetClassDisplayName (Utilities|GetClass (Variables|Default|GetPlacedTower)))))
  (Default|Radial (Variables|Default|GetUI) self _output_get))

(fn Send"Default"toRadialMenu
  (bind _output_get (Variables|Default|SetClass "Default"))
  (Default|Radial (Variables|Default|GetUI) self _output_get))

(fn CreateRadialMenuWidget
  (bind _output_get (Variables|Default|SetCell (Variables|Default|GetCell)))
  (Sprite|SetSpriteColor _output_get (Math|Conversions|ToLinearColor(Color) (Variables|Default|GetActiveCellColor)))
  (Rendering|Components|Sprite|SetSprite (Variables|Default|GetCell) (Variables|Default|GetActiveCellSprite))
  (bind _returnvalue (UserInterface|CreateWidget "/Game/BluePrints/UI/BP_Radial.BP_Radial_C" (Game|GetPlayerController 0)))
  (Variables|Default|SetUI _returnvalue)
  (UserInterface|Viewport|AddtoViewport _returnvalue 0))

(fn CreateObstacleUI
  (bind _returnvalue (UserInterface|CreateWidget "/Game/BluePrints/UI/BP_ObstacleGrid.BP_ObstacleGrid_C" (Game|GetPlayerController 0)))
  (UserInterface|Viewport|AddtoViewport _returnvalue 0))

(fn GetAllTowersandSuspressCollider
  (bind _outactors (Actor|GetAllActorswithInterface "/Game/BluePrints/Interface/BPI_Shoot.BPI_Shoot_C"))
  (for _array_element _outactors
    (Class|BPIShoot|SuppressCollider(Message) _array_element)))

(fn SetColorOfObstacle
  (params (Alpha :type Float%20%28single-precision%29))
  (bind _obstacle (Variables|Default|GetObstacle))
  (bind _spritecolor (Variables|/Script/Paper2D.PaperSpriteComponent|GetSpriteColor _obstacle))
  (bind (_r _g _b) (Math|Color|BreakColor _spritecolor))
  (Sprite|SetSpriteColor _obstacle (Math|Color|MakeColor _r _g _b Alpha)))