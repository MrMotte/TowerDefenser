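; Tower Blueprint for a tower-defense style turret that fires projectiles at enemies in range.
; Clicking or touching the Cone component makes it visible and enables the tower.
; While enabled, every Tick spawns a Projectile at SpawnPoint and shoots it at the first Enemy overlapping Range, with no cooldown.
; A loop over all overlapping enemies is left disconnected.
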(event OnInputTouchBegin(Cone)
  (params (FingerIndex :type ETouchIndex%20Enum :default "Touch1") (TouchedComponent :type Primitive%20Component%20Object%20Reference))
  (Rendering|SetVisibility (Variables|Default|GetCone) true false)
  (CallFunction|EnableTower))

(event OnClicked(Cone)
  (params (TouchedComponent :type Primitive%20Component%20Object%20Reference) (ButtonPressed :type Key%20Structure))
  (Rendering|SetVisibility (Variables|Default|GetCone) true false)
  (CallFunction|EnableTower))

(event Custom|EnableTower
  (Variables|Default|SetEnabled? true))

(event EventBeginPlay)

(event EventTick
  (params (DeltaSeconds :type Float%20%28single-precision%29))
  (bind _range (Variables|Default|GetRange))
  (bind _overlappingactors (Collision|GetOverlappingActors _range "/Game/BluePrints/Enemy.Enemy_C" :!class /Script/Engine.PrimitiveComponent))
  (bind _output (Utilities|Array|Get(acopy) _overlappingactors))
  (if (Variables|Default|GetEnabled?)
    (if (Utilities|IsValid _output)
      (bind _returnvalue (Game|SpawnActorfromClass "/Game/BluePrints/Projectile.Projectile_C" (Transformation|GetWorldTransform (Variables|Default|GetSpawnPoint)) "Undefined" 0 0))
      (Default|Shoot _returnvalue _output))))

(fn ConstructionScript)