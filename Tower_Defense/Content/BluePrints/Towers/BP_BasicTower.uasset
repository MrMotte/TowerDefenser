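; BP_BasicTower is a tower that turns toward and shoots the first hittable actor overlapping its range sphere.
; Each tick it checks that target, smoothly rotates to it and, unless cooling down, plays the fire animation and sound.
; Bullets come from BP_SpawnManager's object pool and receive the target via ShootMessage.
; Construction sets range and scales animation to fire rate using hardcoded timings; interface events show or hide the range sphere.
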(event EventTick
  (params (DeltaSeconds :type Float%20%28single-precision%29))
  ;[1 0.3185 0 1 35] On Tick: Get First Enemy, check if valid, Play Anim and spawn Bullet
  (Variables|Default|SetFirstOverlapActor (Utilities|Array|Get(acopy) (Collision|GetOverlappingActors (Variables|Default|GetCollisionRange) 0 :!class /Script/Engine.PrimitiveComponent)))
  (if (Utilities|IsValidANDImplementInterfaceGetHitted)
    (Utilities|FlowControl|Sequence
      (:then_0
        (Utilities|PlayAnim)
        (Utilities|SpawnBullet)
        (Utilities|FlowControl|Delay (* (Variables|Default|GetE_Rate%20of%20Fire%20in%20sec) 0.6992))
        (Variables|Default|SetJustFired? false))
      (:then_1
        (Utilities|SetTowerLookatEnemy)))))

(event EventShowCollider
  ;[1 0 1 1 35] Interface call: Show Collider
  (Development|SetHiddeninGame (Variables|Default|GetCollisionRange) false false))

(event EventSuspressCollider
  ;[1 0 1 1 35] Interface call: Suspress Collider
  (Development|SetHiddeninGame (Variables|Default|GetCollisionRange) true false))

(fn ConstructionScript
  (Components|Sphere|SetSphereRadius (Variables|Default|GetCollisionRange) (Variables|Default|GetE_Range%20in%20UE%20Units) true)
  (bind _outactors (Actor|GetAllActorsOfClass "/Game/BluePrints/BP_SpawnManager.BP_SpawnManager_C"))
  ;[1 1 1] hardcode anim length
  (Variables|Default|SetBP_SpawnManager (Utilities|Array|Get(acopy) _outactors))
  (Variables|/Script/Engine.SkeletalMeshComponent|SetGlobalAnimRateScale (Variables|Default|GetTowerSkeletel) (/ 1.875 (Variables|Default|GetE_Rate%20of%20Fire%20in%20sec))))

(fn SpawnActorfromPool
  (params (SpawnTransform :type Transform) (ObjectPoolString :type String)))