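; Castle Blueprint that acts as the player's base, tracking a life count and showing it on a text component.
; Any actor overlapping the DeadZone component is destroyed and costs one life, with no filter on actor type.
; The life text refreshes on begin play and after each hit, and the game pauses when life reaches exactly zero.
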(event OnComponentBeginOverlap(DeadZone)
  (params (OverlappedComponent :type Primitive%20Component%20Object%20Reference) (OtherActor :type Actor%20Object%20Reference) (OtherComp :type Primitive%20Component%20Object%20Reference) (OtherBodyIndex :type Integer) (bFromSweep :type Boolean) (SweepResult :type Hit%20Result%20Structure%20%28by%20ref%29))
  (Variables|Default|SetLife (- (Variables|Default|GetLife) 1))
  (Actor|DestroyActor OtherActor)
  (Rendering|Components|TextRender|SetText (Variables|Default|GetLifeCount) (Utilities|Text|ToText(Integer) (Variables|Default|GetLife)))
  (if (== (Variables|Default|GetLife) 0)
    (Game|SetGamePaused true)))

(event EventBeginPlay
  (Rendering|Components|TextRender|SetText (Variables|Default|GetLifeCount) (Utilities|Text|ToText(Integer) (Variables|Default|GetLife))))

(event EventTick
  (params (DeltaSeconds :type Float%20%28single-precision%29)))

(fn ConstructionScript)