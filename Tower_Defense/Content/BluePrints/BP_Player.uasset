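; BP_Player holds the player's Life and XP, apparently as a house that enemies damage, and shows both values as text.
; HitPlayer plays a break sound and damage particles, subtracts Life, refreshes its text and calls CountEnemysLeft on the first BP_EnemySpawner found.
; When Life runs out, a DoOnce clears all widgets and opens BP_GameOver with UI-only input.
; XPEnemyTOUI adds earned XP and updates the EnergyCount text.
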(event EventBeginPlay
  ;[0.06848 0.2384 0.807] Initiate Life Count Text
  (CallFunction|InitiateLifeCountText)
  (bind _output_get (Variables|Default|SetXP (+ (stale EventXPEnemyTOUI XPEarned) (Variables|Default|GetXP))))
  (Rendering|Components|TextRender|SetText (Variables|Default|GetEnergyCount) (Utilities|Text|ToText(Float) _output_get "HalfToEven")))

(event EventXPEnemyTOUI
  (params (XPEarned :type Float%20%28single-precision%29))
  (bind _output_get (Variables|Default|SetXP (+ XPEarned (Variables|Default|GetXP))))
  (Rendering|Components|TextRender|SetText (Variables|Default|GetEnergyCount) (Utilities|Text|ToText(Float) _output_get "HalfToEven")))

(event EventHitPlayer
  (params (Damage :type Float%20%28single-precision%29))
  ;[1 0 1] On hitted by Enemy: Spawn Emitter, Update Life (and Life Text) and Create "GameOver" Widget if Life = 0
  (Audio|PlaySoundatLocation "/Game/Sounds/S_Woordbreak.S_Woordbreak" (Transformation|GetActorLocation self))
  (Variables|Default|SetLife (- (Variables|Default|GetLife) Damage))
  (Effects|SpawnEmitteratLocation "/Game/Particles/House/PS_HouseDamage.PS_HouseDamage" (Transformation|GetWorldLocation (Variables|Default|GetEmitterSpawnLocation)))
  (bind _outactors (Actor|GetAllActorsOfClass "/Game/BluePrints/BP_EnemySpawner.BP_EnemySpawner_C"))
  (Default|CountEnemysLeft (Utilities|Array|Get(acopy) _outactors))
  (CallFunction|UpdateLifeCountText)
  (if (<= (Variables|Default|GetLife) 0.0)
    (Utilities|FlowControl|DoOnce false
      (:Completed
        (Viewport|RemoveAllWidgets)
        (CallFunction|CreateUI"GameOver")))))

(fn ConstructionScript)

(fn InitiateLifeCountText
  (Rendering|Components|TextRender|SetText (Variables|Default|GetLifeCount) (Utilities|Text|ToText(Integer) (Math|Float|Truncate (Variables|Default|GetLife)))))

(fn UpdateLifeCountText
  (Rendering|Components|TextRender|SetText (Variables|Default|GetLifeCount) (Utilities|Text|ToText(Integer) (Math|Float|Truncate (Variables|Default|GetLife)))))

(fn CreateUI"GameOver"
  (bind _returnvalue (Game|GetPlayerController 0))
  (bind _returnvalue_2 (UserInterface|CreateWidget "/Game/BluePrints/UI/BP_GameOver.BP_GameOver_C" _returnvalue))
  (Variables|Default|SetGameOver _returnvalue_2)
  (UserInterface|Viewport|AddtoViewport _returnvalue_2 0)
  (Input|SetInputModeUIOnly _returnvalue _returnvalue_2 "DoNotLock"))