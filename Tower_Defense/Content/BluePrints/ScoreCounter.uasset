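; ScoreCounter is an actor that calculates the player's score and star rating when a level ends.
; LevelHasEnded reads XP, stored as end-of-level energy, and remaining lives from the first BP_Player found, then prints the resulting score.
; CalculateLevelScore weights energy and lives by points-per-unit variables and cascades through score thresholds to award zero to three stars, with ties earning the higher rating.
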(event Custom|LevelHasEnded
  (bind _outactors (Actor|GetAllActorsOfClass "/Game/BluePrints/BP_Player.BP_Player_C"))
  (bind _xp (Default|GetXP (Utilities|Array|Get(acopy) _outactors)))
  (Variables|Default|SetEnergyAtEndOfLevel _xp)
  (Variables|Default|SetLivesLeftAtEndOfLevel (Variables|/Game/BluePrints/BP_Player.BP_Player_C|GetLife (Utilities|Array|Get(acopy) _outactors)))
  (CallFunction|CalculateLevelScore)
  (Development|PrintString (Utilities|String|Append "Score in this level: " (Utilities|String|ToString(Float) (Variables|Default|GetScore)))))

(event EventBeginPlay)

(event Collision|EventActorBeginOverlap
  (params (OtherActor :type Actor%20Object%20Reference)))

(event EventTick
  (params (DeltaSeconds :type Float%20%28single-precision%29)))

(fn ConstructionScript)

(fn CalculateLevelScore
  (bind _output_get (Variables|Default|SetScore (+ (* (Variables|Default|GetEnergyAtEndOfLevel) (Variables|Default|GetPointsAwardedPerEnergy)) (* (Variables|Default|GetLivesLeftAtEndOfLevel) (Variables|Default|GetPointsAwardedPerLife)))))
  (Math|Float|CompareFloat _output_get (Variables|Default|GetScoreNeededFor3Stars)
    (:>
      (Variables|Default|SetStars 3 :!label _label))
    (:==
      (goto _label))
    (:<
      (Math|Float|CompareFloat _output_get (Variables|Default|GetScoreNeededFor2Stars)
        (:>
          (Variables|Default|SetStars 2 :!label _label_2))
        (:==
          (goto _label_2))
        (:<
          (Math|Float|CompareFloat _output_get (Variables|Default|GetScoreNeededFor1Star)
            (:>
              (Variables|Default|SetStars 1 :!label _label_3))
            (:==
              (goto _label_3))
            (:<
              (Variables|Default|SetStars 0))))))))