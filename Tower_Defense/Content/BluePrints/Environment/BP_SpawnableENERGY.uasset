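; BP_SpawnableENERGY is a spawnable energy pickup that the player collects by touch.
; On BeginPlay it starts the Spawn sequence and the endlessly looping Idle sequence, and enables a countdown if Lifetime is positive.
; Tick destroys it when the countdown runs out.
; A touch sends EnergyToAward to the first BP_Player found, through XPEnemyTOUIMessage, then destroys the actor.
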(event EventBeginPlay
  (Sequencer|Player|Play (Variables|/Script/ActorSequence.ActorSequenceComponent|GetSequencePlayer (Variables|Default|GetSpawn)) :!class /Script/MovieScene.MovieSceneSequencePlayer)
  (Class|MovieSceneSequencePlayer|PlayLooping (Variables|/Script/ActorSequence.ActorSequenceComponent|GetSequencePlayer (Variables|Default|GetIdle)) -1)
  (Math|Float|CompareFloat (Variables|Default|GetLifetime) 0.0
    (:>
      (Variables|Default|SetHasLifetime true)
      (Variables|Default|SetCountDownLifetime (Variables|Default|GetLifetime)))
    (:==
      (Variables|Default|SetHasLifetime false :!label _label))
    (:<
      (goto _label))))

(event Collision|EventActorBeginOverlap
  (params (OtherActor :type Actor%20Object%20Reference)))

(event EventTick
  (params (DeltaSeconds :type Float%20%28single-precision%29))
  (if (Variables|Default|GetHasLifetime)
    (Variables|Default|SetCountDownLifetime (- (Variables|Default|GetCountDownLifetime) DeltaSeconds))
    (Math|Float|CompareFloat (Variables|Default|GetCountDownLifetime) 0.0
      (:==
        _)
      (:<
        _))
    (CallFunction|DestroyThis)))

(event EventActorOnInputTouchBegin
  (params (FingerIndex :type ETouchIndex%20Enum :default "Touch1"))
  (CallFunction|AwardEnergy)
  (CallFunction|DestroyThis))

(fn ConstructionScript)

(fn AwardEnergy
  (bind _outactors (Actor|GetAllActorsOfClass "/Game/BluePrints/BP_Player.BP_Player_C"))
  (Class|BPIXP|XPEnemyTOUI(Message) (Utilities|Array|Get(acopy) _outactors) (Variables|Default|GetEnergyToAward)))

(fn DestroyThis
  (Actor|DestroyActor))

(fn PlayAnimation
  (Sequencer|Player|Play (Variables|/Script/ActorSequence.ActorSequenceComponent|GetSequencePlayer (Variables|Default|GetSpawn)) :!class /Script/MovieScene.MovieSceneSequencePlayer))