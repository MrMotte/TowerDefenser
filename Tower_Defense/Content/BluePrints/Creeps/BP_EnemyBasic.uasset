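; Pooled basic creep enemy that follows the BP_Spline path each tick and damages the player on overlap before returning to the pool.
; Wave-supplied stats set life, damage, speed and XP; interface calls apply direct, area and over-time damage, plus freeze-then-slow that also scales animation.
; The damage-over-time loop repeats until death, which plays effects, hides the creep, notifies spawner and player once via DoOnce, then pools it after a delay.
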(event OnComponentBeginOverlap(EnemyBase)
  (params (OverlappedComponent :type Primitive%20Component%20Object%20Reference) (OtherActor :type Actor%20Object%20Reference) (OtherComp :type Primitive%20Component%20Object%20Reference) (OtherBodyIndex :type Integer) (bFromSweep :type Boolean) (SweepResult :type Hit%20Result%20Structure%20%28by%20ref%29))
  ;[0 0 1 1 40] On Overlap Player: Send Damage to Player and destroy self
  (if (Utilities|DoesObjectImplementInterface OtherActor "/Game/BluePrints/Interface/BPI_HittedPlayer.BPI_HittedPlayer_C")
    (Class|BPIHittedPlayer|HitPlayer(Message) OtherActor (Variables|Default|GetE_Damage))
    (Utilities|FlowControl|Delay 0.2)
    (Class|PooledActor|ReturntoPool)))

(event Custom|ResetOnReturnToPool
  ;[1 0 1 1 40] Enemy Death: Spawn Emitter, Set Speed and Visibility, Send death to Player, send XP to XP UI
  (Utilities|FlowControl|DoOnce false) ; enters at Reset
)

(event Custom|GetSpline
  ;[0.06848 0.2384 0.807 1 40] On BeginPlay: Get and store Spline
  (bind _outactors (Actor|GetAllActorsOfClass "/Game/BluePrints/BP_Spline.BP_Spline_C"))
  (Variables|Default|SetStoredSpline (Variables|/Game/BluePrints/BP_Spline.BP_Spline_C|GetSpline (Utilities|Array|Get(acopy) _outactors))))

(event Custom|DotLoop
  ;[1 0 1 1 40] Dot: Get Dot Duration, Damage and Ticks, calculate life and Ticks Dot to end or Enemys death
  (Variables|Default|SetE_Life (- (Variables|Default|GetE_Life) (Variables|Default|GetTickDamage)))
  (Utilities|FlowControl|Delay (Variables|Default|GetIntervall))
  (Variables|Default|SetCountDot (- (Variables|Default|GetCountDot) 1))
  (if (<= (Variables|Default|GetE_Life) 0.0)
    (CallFunction|EnemyDeath)
    (else
      (CallFunction|DotLoop))))

(event Custom|Dot
  (params (DotDuration :type Float%20%28single-precision%29) (DotDamage :type Float%20%28single-precision%29) (DotTicks :type Integer))
  (bind (_intervall _damage_per_tick) (Utilities|CalculateIntervallandDamagePerTick DotDuration DotDamage DotTicks))
  ;[1 0 1 1 40] Dot: Get Dot Duration, Damage and Ticks, calculate life and Ticks Dot to end or Enemys death
  (Variables|Default|SetCountDot DotTicks)
  (Variables|Default|SetIntervall _intervall)
  (Variables|Default|SetTickDamage _damage_per_tick)
  (Variables|Default|SetE_Life (- (Variables|Default|GetE_Life) (Variables|Default|GetTickDamage)))
  (Utilities|FlowControl|Delay (Variables|Default|GetIntervall))
  (Variables|Default|SetCountDot (- (Variables|Default|GetCountDot) 1))
  (if (<= (Variables|Default|GetE_Life) 0.0)
    (CallFunction|EnemyDeath)
    (else
      (CallFunction|DotLoop))))

(event Custom|EnemyDeath
  (bind _particlespawnlocation (Variables|Default|GetParticleSpawnLocation))
  (bind _skeletalmesh (Variables|Default|GetSkeletalMesh))
  (bind _returnvalue (Transformation|GetWorldLocation _particlespawnlocation))
  ;[1 0 1 1 40] Enemy Death: Spawn Emitter, Set Speed and Visibility, Send death to Player, send XP to XP UI
  (Audio|SpawnSoundatLocation (Variables|Default|GetDeathSound_Creep) _returnvalue)
  (Effects|SpawnEmitteratLocation "/Game/Particles/Creeps/PS_CreepDeath.PS_CreepDeath" _returnvalue)
  (Variables|Default|SetE_Speed 0.005)
  (Rendering|SetVisibility (Variables|Default|GetEnemyBase) false false)
  (Collision|SetCollisionEnabled (Variables|Default|GetEnemyBase) "NoCollision")
  (Rendering|SetVisibility _skeletalmesh false false)
  (Collision|SetCollisionEnabled _skeletalmesh "NoCollision")
  (bind _outactors (Actor|GetAllActorsOfClass "/Game/BluePrints/BP_EnemySpawner.BP_EnemySpawner_C"))
  (Utilities|FlowControl|Sequence
    (:then_0
      (Utilities|FlowControl|Delay 4.05)
      (Class|PooledActor|ReturntoPool))
    (:then_1
      (Utilities|FlowControl|DoOnce false
        (:Completed
          (Default|CountEnemysLeft (Utilities|Array|Get(acopy) _outactors))
          (bind _outactors_2 (Actor|GetAllActorsOfClass "/Game/BluePrints/BP_Player.BP_Player_C"))
          (Default|XPEnemyTOUI (Utilities|Array|Get(acopy) _outactors_2) (Variables|Default|GetE_XPEarn)))))))

(event Custom|Slow
  (params (SlowDuration :type Float%20%28single-precision%29) (FreezDuration :type Float%20%28single-precision%29) (SpeedMultiplier :type Float%20%28single-precision%29))
  ;[1 0 1 1 40] Slow: Get Slow and Freeze Values, calculate and execute first freeze (if valid) and then slow
  (Utilities|InitiateVariables SlowDuration FreezDuration SpeedMultiplier)
  (if (> (Variables|Default|GetFreeze%20Duration) 0.01)
    (Variables|Default|SetE_Speed 0.0)
    (Variables|/Script/Engine.SkeletalMeshComponent|SetGlobalAnimRateScale (Variables|Default|GetSkeletalMesh) 0.0)
    (Utilities|FlowControl|Delay (Variables|Default|GetFreeze%20Duration))
    (Variables|/Script/Engine.SkeletalMeshComponent|SetGlobalAnimRateScale (Variables|Default|GetSkeletalMesh) (Variables|Default|GetE_AnimSpeed)))
  (if (> (Variables|Default|GetSlow%20Duration) 0.0)
    (Variables|Default|SetE_Speed (Utilities|CalculateSlowedSpeed))
    (Variables|/Script/Engine.SkeletalMeshComponent|SetGlobalAnimRateScale (Variables|Default|GetSkeletalMesh) (Utilities|CalculateAnimationSpeed))
    (Utilities|FlowControl|Delay (Variables|Default|GetSlow%20Duration))
    (Variables|Default|SetE_Speed (Variables|Default|GetDefaultSpeed))
    (Variables|/Script/Engine.SkeletalMeshComponent|SetGlobalAnimRateScale (Variables|Default|GetSkeletalMesh) (Variables|Default|GetE_AnimSpeed))))

(event EventGetVarfromWave
  (params (E_Life :type Float%20%28single-precision%29) (E_Damage :type Float%20%28single-precision%29) (E_Speed :type Float%20%28single-precision%29) (E_XPEarn :type Float%20%28single-precision%29))
  (Variables|Default|SetE_Life E_Life)
  (Variables|Default|SetE_Damage E_Damage)
  (Variables|Default|SetE_Speed E_Speed)
  (Variables|Default|SetE_XPEarn E_XPEarn)
  (Variables|Default|SetDefaultSpeed E_Speed))

(event EventEVENTonPoolEndPlay
  (CallFunction|ResetonReturntoPool))

(event EventEVENTonPoolBeginPlay
  (Utilities|FlowControl|Sequence
    (:then_0
      (Variables|Default|SetStoredDistance 0.0)
      (Variables|Default|SetCountDot 0)
      (Variables|Default|SetTickDamage 0.0)
      (Variables|Default|SetSlow%20Duration 0.0)
      (Variables|Default|SetFreeze%20Duration 0.0)
      (Variables|Default|SetSpeed%20Multiplier 1.0)
      (if (Variables|Default|GetE_EnableAnim?)
        _))
    (:then_1
      (CallFunction|GetSpline))))

(event EventDamageValue
  (params (Damage :type Float%20%28single-precision%29))
  ;[1 0 1 1 40] On Interface call: Get Direct Damage and calculate life
  (bind _output_get (Variables|Default|SetE_Life (- (Variables|Default|GetE_Life) Damage)))
  (if (<= _output_get 0.0)
    (CallFunction|EnemyDeath)))

(event EventTick
  (params (DeltaSeconds :type Float%20%28single-precision%29))
  (bind (_returnvalue _returnvalue2) (Utilities|GetSplineRotationandLocation))
  ;[0 1 0 1 40] On Tick: Move on Spline
  (Variables|Default|SetStoredDistance (Utilities|CalculateNewPositiononSpline))
  (Transformation|SetWorldLocationAndRotation (Variables|Default|GetDefaultSceneRoot) _returnvalue _returnvalue2 false false))

(event EventAreaDamage
  (params (Damage :type Float%20%28single-precision%29))
  ;[1 0 1 1 40] On Interface call: Get Area Damage and calculate life
  (bind _output_get (Variables|Default|SetE_Life (- (Variables|Default|GetE_Life) Damage)))
  (if (<= _output_get 0.0)
    (CallFunction|EnemyDeath)))

(event EventDamageOverTime
  (params (DotDuration :type Float%20%28single-precision%29) (DotDamage :type Float%20%28single-precision%29) (DOTTicks :type Integer) (SlowDuration :type Float%20%28single-precision%29) (SpeedMultiplier :type Float%20%28single-precision%29) (FreezDuration :type Float%20%28single-precision%29))
  ;[1 0 1 1 40] On Interface call: Get Damage Over Time and distribiute Value to Slow and Dot Events
  (Utilities|FlowControl|Sequence
    (:then_0
      (if (> DotDuration 0.0)
        (CallFunction|Dot DotDuration DotDamage DOTTicks)))
    (:then_1
      (if (or (> SlowDuration 0.0) (> FreezDuration 0.0))
        (CallFunction|Slow SlowDuration FreezDuration SpeedMultiplier)))))

(event EventBeginPlay
  ;[0.06848 0.2384 0.807 1 40] On BeginPlay: Get and store Spline
  (bind _outactors (Actor|GetAllActorsOfClass "/Game/BluePrints/BP_Spline.BP_Spline_C"))
  (Variables|Default|SetStoredSpline (Variables|/Game/BluePrints/BP_Spline.BP_Spline_C|GetSpline (Utilities|Array|Get(acopy) _outactors))))

(fn ConstructionScript)