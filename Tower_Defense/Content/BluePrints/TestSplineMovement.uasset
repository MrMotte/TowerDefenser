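; Test actor that moves itself along the spline of a BP_Spline actor placed in the level.
; On BeginPlay it caches the Spline component from the first BP_Spline found.
; Each Tick increments Speed, which serves as distance travelled, and sets the root's world location and rotation from the spline at that distance.
; The step ignores delta time, so movement rate depends on frame rate.
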(event EventTick
  (params (DeltaSeconds :type Float%20%28single-precision%29))
  (bind _storedspline (Variables|Default|GetStoredSpline))
  (Variables|Default|SetSpeed (+ (Variables|Default|GetSpeed) 1.0))
  (Transformation|SetWorldLocationAndRotation (Variables|Default|GetDefaultSceneRoot) (Spline|GetLocationatDistanceAlongSpline _storedspline (Variables|Default|GetSpeed) "World") (Spline|GetRotationatDistanceAlongSpline _storedspline (Variables|Default|GetSpeed) "World") false false))

(event EventBeginPlay
  (bind _outactors (Actor|GetAllActorsOfClass "/Game/BluePrints/BP_Spline.BP_Spline_C"))
  (Variables|Default|SetStoredSpline (Variables|/Game/BluePrints/BP_Spline.BP_Spline_C|GetSpline (Utilities|Array|Get(acopy) _outactors))))

(fn ConstructionScript)