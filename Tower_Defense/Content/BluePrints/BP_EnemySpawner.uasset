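; BP_EnemySpawner is an enemy spawner actor that runs timed waves and shows the win screen once every enemy is counted off.
; After BeginPlay, it totals enemies across the Waves array and starts a delay-driven recursive spawn loop, alongside a timer that advances waves.
; Each enemy spawns at the spawner's transform and receives stored waypoints through a GetArray message.
; CountEnemysLeft decrements the total, creating BP_Win with UI-only input at zero.
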(event Custom|CountEnemys
  (for _array_element (Variables|Default|GetWaves)
    (Variables|Default|SetGetEnemySum (+ (.Amount (Utilities|Struct|BreakWave _array_element)) (Variables|Default|GetGetEnemySum))))
  (Development|PrintString "enemysum counted"))

(event Custom|SpawnAgain
  (bind _waves (Variables|Default|GetWaves))
  (bind _currentwave (Variables|Default|GetCurrentWave))
  (bind _output (Utilities|Array|Get(acopy) _waves _currentwave))
  (bind (_amount _class _durationbetweenenemyspawn _durationbetweenwaves) (Utilities|Struct|BreakWave _output))
  (if (> (Variables|Default|GetMaxAmount) 0)
    (bind _returnvalue (Game|SpawnActorfromClass _class (Transformation|GetWorldTransform (Variables|Default|GetDefaultSceneRoot)) "Undefined" 0 0))
    (Class|BPIWaypointInterface|GetArray(Message) _returnvalue (Variables|Default|GetStoreWaypoints))
    (Utilities|FlowControl|Delay _durationbetweenenemyspawn)
    (Variables|Default|SetMaxAmount (- (Variables|Default|GetMaxAmount) 1))
    (CallFunction|SpawnAgain)))

(event Custom|TimeTillNext
  (Utilities|FlowControl|Delay (.DurationBetweenWaves (Utilities|Struct|BreakWave (Utilities|Array|Get(acopy) (Variables|Default|GetWaves) (Variables|Default|GetCurrentWave)))))
  (if (< (Variables|Default|GetCurrentWave) (- (Variables|Default|GetLength) 1))
    (Variables|Default|SetCurrentWave (+ (Variables|Default|GetCurrentWave) 1))
    (CallFunction|InitiateWave)))

(event Custom|InitiateWave
  (bind _waves (Variables|Default|GetWaves))
  (Variables|Default|SetLength (Utilities|Array|Length _waves))
  (Variables|Default|SetMaxAmount (.Amount (Utilities|Struct|BreakWave (Utilities|Array|Get(acopy) _waves (Variables|Default|GetCurrentWave)))))
  (CallFunction|SpawnAgain)
  (CallFunction|TimeTillNext))

(event EventBeginPlay
  (Utilities|FlowControl|Delay 1.0)
  (CallFunction|InitiateWave)
  (CallFunction|CountEnemys))

(event Collision|EventActorBeginOverlap
  (params (OtherActor :type Actor%20Object%20Reference)))

(event EventTick
  (params (DeltaSeconds :type Float%20%28single-precision%29)))

(event EventGetArray
  (params (WaypointIN :type Array%20of%20Transforms))
  (Variables|Default|SetStoreWaypoints WaypointIN))

(event EventCountEnemysLeft
  (bind _returnvalue (Game|GetPlayerController 0))
  ;[1 1 1] Count Enemys left and add WIN ui to vieport
  (Variables|Default|SetGetEnemySum (- (Variables|Default|GetGetEnemySum) 1))
  (if (== (Variables|Default|GetGetEnemySum) 0)
    (bind _returnvalue_2 (UserInterface|CreateWidget "/Game/BluePrints/BP_Win.BP_Win_C" _returnvalue))
    (Variables|Default|SetWin _returnvalue_2)
    (UserInterface|Viewport|AddtoViewport _returnvalue_2 0)
    (Input|SetInputModeUIOnly _returnvalue _returnvalue_2 "DoNotLock")))

(fn ConstructionScript)