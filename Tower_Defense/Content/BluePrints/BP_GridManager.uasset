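; BP_GridManager is a utility actor that builds and manages a square grid of BP_GridField actors.
; RunGrid spawns fields from its own location using modulo and division for spacing, looping from index 1, so the origin cell is skipped.
; Separate events attach all fields in the level to the manager, detach them, or destroy them.
; Deletion uses a Safety countdown as a double-click guard, and each operation prints a completion message.
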(event Custom|RunGrid
  (bind _size (Variables|Default|GetSize))
  (bind _size_2 (Variables|Default|GetSize))
  (bind _blockspacing (Variables|Default|GetBlockSpacing))
  (for _index (range 1 (- (* _size _size) 1)) ; Loop to spawn each block
    (Game|SpawnActorfromClass "/Game/BluePrints/BP_GridField.BP_GridField_C" (Math|Transform|MakeTransform (.Location (Math|Transform|BreakTransform (Math|Conversions|ToTransform(Vector) (+ (Math|Vector|MakeVector (* (Math|Integer|%(Integer) _index _size_2) _blockspacing) (* (/ _index _size_2) _blockspacing) 0.0) (Transformation|GetActorLocation))))) (.Rotation (Math|Transform|BreakTransform (Math|Conversions|ToTransform(Vector) (+ (Math|Vector|MakeVector (* (Math|Integer|%(Integer) _index _size_2) _blockspacing) (* (/ _index _size_2) _blockspacing) 0.0) (Transformation|GetActorLocation))))) (Variables|Default|GetScale)) "AlwaysSpawn" 0 0))
  (Development|PrintString "Create Grid Complete"))

(event Custom|Delete%20Grid%20double%20click%20for%20safety
  (Variables|Default|Setsafety (- (Variables|Default|Getsafety) 1))
  (if (== (Variables|Default|Getsafety) 0)
    (bind _outactors (Actor|GetAllActorsOfClass "/Game/BluePrints/BP_GridField.BP_GridField_C"))
    (for _array_element _outactors
      (Actor|DestroyActor _array_element))
    (Variables|Default|Setsafety 2)
    (Development|PrintString "Delete Complete")))

(event Custom|DetachAllGridFields
  (bind _outactors (Actor|GetAllActorsOfClass "/Game/BluePrints/BP_GridField.BP_GridField_C"))
  (for _array_element _outactors
    (Transformation|DetachFromActor _array_element "KeepWorld" "KeepRelative" "KeepRelative"))
  (Development|PrintString "Detach Complete"))

(event Custom|AttachAllFields
  (bind _outactors (Actor|GetAllActorsOfClass "/Game/BluePrints/BP_GridField.BP_GridField_C"))
  (for _array_element _outactors
    (Transformation|AttachActorToActor _array_element self "None" "KeepWorld" "KeepRelative" "KeepRelative" false))
  (Development|PrintString "Attach Complete"))

(event Collision|EventActorBeginOverlap
  (params (OtherActor :type Actor%20Object%20Reference)))

(event EventTick
  (params (DeltaSeconds :type Float%20%28single-precision%29)))

(event EventBeginPlay)

(fn ConstructionScript)