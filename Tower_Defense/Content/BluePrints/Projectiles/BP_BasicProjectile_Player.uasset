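; Player projectile that can home in on an enemy and deals direct, area and damage-over-time/slow/freeze effects.
; Shoot sets the homing target, while the construction script applies configured speed and AOE radius.
; On overlap it hides itself and messages the hit actor, then optionally messages actors inside the AOE sphere.
; It self-destructs on impact, briefly delayed for area effects, or after a three-second lifetime.
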(event OnComponentBeginOverlap(Bullet)
  (params (OverlappedComponent :type Primitive%20Component%20Object%20Reference) (OtherActor :type Actor%20Object%20Reference) (OtherComp :type Primitive%20Component%20Object%20Reference) (OtherBodyIndex :type Integer) (bFromSweep :type Boolean) (SweepResult :type Hit%20Result%20Structure%20%28by%20ref%29))
  (bind _aoecollision (Variables|Default|GetAOECollision))
  (bind _overlappingactors (Collision|GetOverlappingActors _aoecollision 0 :!class /Script/Engine.PrimitiveComponent))
  ;[1 1 1] Event Begin Overlap (Bullet)
  (Rendering|SetVisibility (Variables|Default|GetBullet) false false)
  (Rendering|SetVisibility (Variables|Default|GetProjectileParticle) false false)
  (Class|BPIGetHitted|DamageValue(Message) OtherActor (Variables|Default|GetE_Damage))
  (Utilities|FlowControl|Sequence
    (:then_0
      (if (not (or (Variables|Default|GetE_ActivateAOEDamage?) (Variables|Default|GetE_ActivateDot|SlowOrFreeze?)))
        (Actor|DestroyActor)))
    (:then_1
      (if (Variables|Default|GetE_ActivateAOEDamage?)
        (for _array_element _overlappingactors
          (if (Utilities|DoesObjectImplementInterface _array_element "/Game/BluePrints/BPI_GetHitted.BPI_GetHitted_C")
            (Class|BPIGetHitted|AreaDamage(Message) _array_element (Variables|Default|GetE_AOEDamage))
            (Utilities|FlowControl|Delay 0.2)
            (Actor|DestroyActor)))))
    (:then_2
      (if (Variables|Default|GetE_ActivateDot|SlowOrFreeze?)
        (for _array_element_2 _overlappingactors
          (Class|BPIGetHitted|DamageOverTime(Message) _array_element_2 (Variables|Default|GetE_DOTDuration) (Variables|Default|GetE_DOTDamage) (Variables|Default|GetE_DOTTicks) (Variables|Default|GetE_SlowDuration) (Variables|Default|GetE_SlowSpeedMultiplier) (Variables|Default|GetE_FreezeDuration))
          (Utilities|FlowControl|Delay 0.2)
          (Actor|DestroyActor))))))

(event EventBeginPlay
  ;[0.3125 0.3125 0.3125] Destroy Actor after 3 seconds
  (Utilities|FlowControl|Delay 3.0)
  (Actor|DestroyActor))

(event EventShoot
  (params (Enemy :type Actor%20Object%20Reference))
  (bind _projectilemovement (Variables|Default|GetProjectileMovement))
  ;[1 1 1] Event Shoot
  (if (Utilities|IsValid Enemy)
    (Variables|/Script/Engine.ProjectileMovementComponent|SetHomingTargetComponent _projectilemovement (Variables|/Script/Engine.Actor|GetRootComponent Enemy))
    (Variables|/Script/Engine.ProjectileMovementComponent|SetbIsHomingProjectile _projectilemovement true)
    (Variables|/Script/Engine.ProjectileMovementComponent|SetHomingAccelerationMagnitude _projectilemovement 1e+04)))

(fn ConstructionScript
  (bind _projectilemovement (Variables|Default|GetProjectileMovement))
  (bind _e_projectilespeed (Variables|Default|GetE_ProjectileSpeed))
  (Variables|/Script/Engine.ProjectileMovementComponent|SetMaxSpeed _projectilemovement _e_projectilespeed)
  (Variables|/Script/Engine.ProjectileMovementComponent|SetInitialSpeed _projectilemovement _e_projectilespeed)
  (Components|Sphere|SetSphereRadius (Variables|Default|GetAOECollision) (Variables|Default|GetE_AOERange) true))