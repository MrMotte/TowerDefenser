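; BP_SpawnableENERGY is a touch-collected energy pickup that rewards the player when tapped.
; On InputTouchBegin it passes EnergyToAward to the first BP_Player found via GetAllActorsOfClass, using XPEnemyTOUIMessage, then destroys itself.
; PlayAnimation plays the actor's ActorSequence, but nothing in this Blueprint calls it.
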(event EventBeginPlay)

(event Collision|EventActorBeginOverlap
  (params (OtherActor :type Actor%20Object%20Reference)))

(event EventTick
  (params (DeltaSeconds :type Float%20%28single-precision%29)))

(event EventActorOnInputTouchBegin
  (params (FingerIndex :type ETouchIndex%20Enum :default "Touch1"))
  (CallFunction|AwardEnergy)
  (CallFunction|DestroyThis))

(fn ConstructionScript)

(fn AwardEnergy
  (bind _outactors (Actor|GetAllActorsOfClass "/Game/BluePrints/BP_Player.BP_Player_C"))
  (Class|BPIXP|XPEnemyTOUI(Message) (Utilities|Array|Get(acopy) _outactors) (Variables|Default|GetEnergyToAward)))

(fn DestroyThis
  (Actor|DestroyActor))

(fn PlayAnimation
  (Sequencer|Player|Play (Variables|/Script/ActorSequence.ActorSequenceComponent|GetSequencePlayer (Variables|Default|GetActorSequence)) :!class /Script/MovieScene.MovieSceneSequencePlayer))