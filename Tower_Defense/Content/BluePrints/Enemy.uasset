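; Enemy actor that travels along a supplied list of waypoints and takes hits through a box overlap.
; GetArray receives the waypoints, and the Construction Script calls Move, which waits briefly before starting movement.
; MoveAgain slides the root component to each waypoint over a fixed time, re-calling itself until the array ends.
; Each overlap destroys the other actor and decrements Life, or destroys the enemy if Life is already zero.
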(event OnComponentBeginOverlap(Box)
  (params (OverlappedComponent :type Primitive%20Component%20Object%20Reference) (OtherActor :type Actor%20Object%20Reference) (OtherComp :type Primitive%20Component%20Object%20Reference) (OtherBodyIndex :type Integer) (bFromSweep :type Boolean) (SweepResult :type Hit%20Result%20Structure%20%28by%20ref%29))
  (if (== (Variables|Default|GetLife) 0)
    (Actor|DestroyActor OtherActor)
    (Actor|DestroyActor)
    (else
      (Variables|Default|SetLife (- (Variables|Default|GetLife) 1))
      (Actor|DestroyActor OtherActor))))

(event Custom|move
  (bind _waypointarray (Variables|Default|GetWaypointArray))
  (Utilities|FlowControl|Delay 1.0)
  (Components|MoveComponentTo (Variables|Default|GetDefaultSceneRoot) (.Location (Math|Transform|BreakTransform (Utilities|Array|Get(acopy) _waypointarray (Variables|Default|GetCount)))) "0, 0, 0" false false 3.0 false)
  (Variables|Default|SetCount (+ (Variables|Default|GetCount) 1))
  (if (not (== (Variables|Default|GetCount) (Utilities|Array|Length _waypointarray)))
    (CallFunction|MoveAgain)))

(event Custom|MoveAgain
  (bind _waypointarray (Variables|Default|GetWaypointArray))
  (Components|MoveComponentTo (Variables|Default|GetDefaultSceneRoot) (.Location (Math|Transform|BreakTransform (Utilities|Array|Get(acopy) _waypointarray (Variables|Default|GetCount)))) "0, 0, 0" false false 3.0 false)
  (Variables|Default|SetCount (+ (Variables|Default|GetCount) 1))
  (if (not (== (Variables|Default|GetCount) (Utilities|Array|Length _waypointarray)))
    (CallFunction|MoveAgain)))

(event EventBeginPlay)

(event Collision|EventActorBeginOverlap
  (params (OtherActor :type Actor%20Object%20Reference)))

(event EventGetArray
  (params (WaypointIN :type Array%20of%20Transforms))
  (Variables|Default|SetWaypointArray WaypointIN))

(event EventTick
  (params (DeltaSeconds :type Float%20%28single-precision%29)))

(fn ConstructionScript
  (CallFunction|Move))