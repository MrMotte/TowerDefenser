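; BP_SpawnManager spawns the player's projectiles (basic, fire, ice and range, plus upgraded variants) from object pools.
; SpawnOneShittyActor switches on a pool name string to choose the matching pool.
; Each case passes that pool and the given transform to SpawnNode, which wraps SpawnActorFromPool, and the spawned actor is returned.
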(fn ConstructionScript)

(fn SpawnOneShittyActor
  (params (SpawnTransform :type Transform) (ObjectPoolString :type String))
  (switch string ObjectPoolString
    (:BP_BasicProjectile_Player_C
      (bind _returnvalue (Utilities|SpawnNode (Variables|Default|GetBPC_Basic_Projectile) SpawnTransform))
      (Variables|Default|SetSpawnedActor _returnvalue))
    (:BP_FireProjectile_Player_C
      (bind _returnvalue_2 (Utilities|SpawnNode (Variables|Default|GetBPC_Fire_Projectile) SpawnTransform))
      (Variables|Default|SetSpawnedActor _returnvalue_2))
    (:BP_FireUpgradeProjectile_Player_C
      (bind _returnvalue_3 (Utilities|SpawnNode (Variables|Default|GetBPC_FireUP_Projectile) SpawnTransform))
      (Variables|Default|SetSpawnedActor _returnvalue_3))
    (:BP_IceProjectile_Player_C
      (bind _returnvalue_4 (Utilities|SpawnNode (Variables|Default|GetBPC_Ice_Projectile) SpawnTransform))
      (Variables|Default|SetSpawnedActor _returnvalue_4))
    (:BP_IceUpgradeProjectile_Player_C
      (bind _returnvalue_5 (Utilities|SpawnNode (Variables|Default|GetBPC_IceUP_Projectile) SpawnTransform))
      (Variables|Default|SetSpawnedActor _returnvalue_5))
    (:BP_RangeProjectile_Player_C
      (bind _returnvalue_6 (Utilities|SpawnNode (Variables|Default|GetBPC_Range_Projectile) SpawnTransform))
      (Variables|Default|SetSpawnedActor _returnvalue_6))
    (:BP_RangeUpgradeProjectile_Player_C
      (bind _returnvalue_7 (Utilities|SpawnNode (Variables|Default|GetBPC_RangeUP_Projectile) SpawnTransform))
      (Variables|Default|SetSpawnedActor _returnvalue_7)))
  (return (Variables|Default|GetSpawnedActor)))