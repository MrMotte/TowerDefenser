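; BP_Character is a character Blueprint whose visible logic handles retrying a level and going to level selection.
; Its TryAgain and LevelSelction events each clear all widgets, then create a BP_LoadingScreen widget and add it to the viewport.
; Each event then calls the matching function on that loading screen, passing the architecture and gameplay level names.
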(event Custom|TryAgain
  (Viewport|RemoveAllWidgets)
  (bind _returnvalue (UserInterface|CreateWidget "/Game/BluePrints/UI/BP_LoadingScreen.BP_LoadingScreen_C"))
  (UserInterface|Viewport|AddtoViewport _returnvalue 0)
  (Default|TryAgain _returnvalue (Variables|Default|GetLevelNameArchitecture) (Variables|Default|GetLevelNameGameplay)))

(event Custom|LevelSelction
  (Viewport|RemoveAllWidgets)
  (bind _returnvalue (UserInterface|CreateWidget "/Game/BluePrints/UI/BP_LoadingScreen.BP_LoadingScreen_C"))
  (UserInterface|Viewport|AddtoViewport _returnvalue 0)
  (Default|LevelSelection _returnvalue (Variables|Default|GetLevelNameArchitecture) (Variables|Default|GetLevelNameGameplay)))

(fn ConstructionScript)