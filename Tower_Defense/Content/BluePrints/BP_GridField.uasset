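; BP_GridField is a grid cell for tower placement, with a touchable Cell component and a reference to its placed tower.
; Touching the cell only checks whether PlacedTower is valid, with no action following either result.
; Disconnected logic would open a BP_Radial widget for non-obstacle cells, or spawn a single BP_BasicTower at the cell's root and store it.
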(event OnInputTouchBegin(Cell)
  (params (FingerIndex :type ETouchIndex%20Enum :default "Touch1") (TouchedComponent :type Primitive%20Component%20Object%20Reference))
  (Utilities|IsValid (Variables|Default|GetPlacedTower)))

(event EventBeginPlay)

(event Collision|EventActorBeginOverlap
  (params (OtherActor :type Actor%20Object%20Reference)))

(event EventTick
  (params (DeltaSeconds :type Float%20%28single-precision%29)))

(fn ConstructionScript)