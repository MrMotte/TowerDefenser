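; BP_BasicTower is a tower that automatically shoots at enemies inside its range sphere.
; The construction script sizes the sphere from the range variable and sets the actor tick interval to the fire rate, so Tick itself paces the shots.
; Each tick, it takes the first overlapping BP_EnemyBasic, checks for BPI_GetHitted, spawns the configured projectile at SpawnPoint and passes it that enemy through ShootMessage.
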(event EventTick
  (params (DeltaSeconds :type Float%20%28single-precision%29))
  (bind _collisionrange (Variables|Default|GetCollisionRange))
  (bind _overlappingactors (Collision|GetOverlappingActors _collisionrange "/Game/BluePrints/BP_EnemyBasic.BP_EnemyBasic_C" :!class /Script/Engine.PrimitiveComponent))
  (bind _output (Utilities|Array|Get(acopy) _overlappingactors))
  ;[1 1 1] get enemys in range
  (if (Utilities|IsValid _output)
    ;[1 1 1] spawn bullet
    (if (Utilities|DoesObjectImplementInterface _output "/Game/BluePrints/BPI_GetHitted.BPI_GetHitted_C")
      (bind _returnvalue (Game|SpawnActorfromClass (Variables|Default|GetE_ProjectileClass) (Transformation|GetWorldTransform (Variables|Default|GetSpawnPoint)) "Undefined" 0 0))
      ;[1 1 1] send enemy in range to bullet
      (Class|BPIShoot|Shoot(Message) _returnvalue _output))))

(fn ConstructionScript
  (Components|Sphere|SetSphereRadius (Variables|Default|GetCollisionRange) (Variables|Default|GetE_Range%20in%20UE%20Units) true)
  (Actor|Tick|SetActorTickInterval (Variables|Default|GetE_Rate%20of%20Fire%20in%20sec)))