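; EnemySpawn is a spawner actor that endlessly spawns enemies at its own transform and hands each one a stored waypoint list.
; GetArray stores incoming waypoints, and BeginPlay starts the loop after a short delay.
; Spawn waits for Speed, spawns an Enemy, then passes it the waypoints via GetArrayMessage after a brief delay.
; It shrinks Speed slightly and calls itself again, so spawns steadily accelerate.
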(event Custom|Spawn
  (Utilities|FlowControl|Delay (Variables|Default|GetSpeed))
  (bind _returnvalue (Game|SpawnActorfromClass "/Game/BluePrints/Enemy.Enemy_C" (Transformation|GetWorldTransform (Variables|Default|GetDefaultSceneRoot)) "Undefined" 0 0))
  (Utilities|FlowControl|Delay 0.1)
  (Class|WaypointInterface|GetArray(Message) _returnvalue (Variables|Default|GetStoreWaypoints))
  (Variables|Default|SetSpeed (* (Variables|Default|GetSpeed) 0.98))
  (CallFunction|Spawn))

(event EventBeginPlay
  (Utilities|FlowControl|Delay 1.0)
  (CallFunction|Spawn))

(event Collision|EventActorBeginOverlap
  (params (OtherActor :type Actor%20Object%20Reference)))

(event EventTick
  (params (DeltaSeconds :type Float%20%28single-precision%29)))

(event EventGetArray
  (params (WaypointIN :type Array%20of%20Transforms))
  (Variables|Default|SetStoreWaypoints WaypointIN))

(fn ConstructionScript)